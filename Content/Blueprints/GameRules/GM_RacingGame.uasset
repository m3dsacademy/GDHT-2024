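; Game mode for the racing game that opens the main menu and spawns local players.
; On BeginPlay it shows and focuses W_MainMenu, then after a short delay creates a local player per connected input device, only when at least two are detected.
; Each starting player is added to PlayerList, and its BPC_RacingGame controller receives that list index through ConnectToGameMessage.
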(event `self.ReceiveBeginPlay`
  (bind _returnvalue (`|CreateWidget` "/Game/UI/W_MainMenu.W_MainMenu_C" (`GameplayStatics.GetPlayerController` 0)))
  (`UserWidget.AddToViewport` _returnvalue 0)
  (bind _output_get (set `self.MainMenu` _returnvalue))
  (`Widget.SetFocus` _output_get)
  (`/Engine/EditorBlueprintResources/StandardMacros.DoOnce` false
    (:`Completed`
      (`KismetSystemLibrary.Delay` 0.2)
      (`self.StartLoadingPlayers`))))

(event `self.HandleStartingNewPlayer`
  (params (NewPlayer :type "PlayerController Object Reference"))
  (bind _returnvalue (`KismetArrayLibrary.Array_Add` (`self.PlayerList`) NewPlayer))
  (bind _asbpc_racing_game (cast `/Game/Blueprints/Input/Controllers/BPC_RacingGame` NewPlayer))
  (message `/Game/Blueprints/BPI_StartGame.ConnectToGame` _asbpc_racing_game _returnvalue))

(event `StartLoadingPlayers`
  (bind (_outinputdevices _returnvalue) (`InputDeviceLibrary.GetAllConnectedInputDevices`))
  (if (>= _returnvalue 2)
    (for _index (range _returnvalue)
      (`GameplayStatics.CreatePlayer` _index))))

(fn `UserConstructionScript`)