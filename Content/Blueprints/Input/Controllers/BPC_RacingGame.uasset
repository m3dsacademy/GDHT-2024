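; Per-player controller for a racing game of up to four players, covering menu car selection through in-race HUD and camera.
; Player index picks team color, menu overlay, PlayerStart and CineCamera by array position.
; Readying up spawns and possesses the chosen car, attaches the camera to its spring arm and swaps input contexts.
; StartGame adds isometric controls and a speed/gear HUD; camera toggle flips between pawn and cine views.
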(event `self.ReceiveBeginPlay`
  (`WidgetBlueprintLibrary.SetInputMode_GameAndUIEx` self null)
  (bind _asgm_racing_game (cast `/Game/Blueprints/GameRules/GM_RacingGame` (`GameplayStatics.GetGameMode`)))
  (set `self.Main Menu` (`/Game/Blueprints/GameRules/GM_RacingGame.MainMenu` _asgm_racing_game)))

(event `EnhancedInput|/Game/Blueprints/Input/Actions/IA_NextCar`
  (params (ActionValue :type Boolean) (ElapsedSeconds :type "Float (double-precision)") (TriggeredSeconds :type "Float (double-precision)") (InputAction :type "InputAction Object Reference" :default "/Game/Blueprints/Input/Actions/IA_NextCar.IA_NextCar"))
  (:`Started`
    (`/Game/UI/W_MainMenu.ChangeCar` (`self.Main Menu`) (`self.iPlayerIndex`) true)))

(event `EnhancedInput|/Game/Blueprints/Input/Actions/IA_PreviousCar`
  (params (ActionValue :type Boolean) (ElapsedSeconds :type "Float (double-precision)") (TriggeredSeconds :type "Float (double-precision)") (InputAction :type "InputAction Object Reference" :default "/Game/Blueprints/Input/Actions/IA_PreviousCar.IA_PreviousCar"))
  (:`Started`
    (`/Game/UI/W_MainMenu.ChangeCar` (`self.Main Menu`) (`self.iPlayerIndex`) false)))

(event `EnhancedInput|/Game/Blueprints/Input/Actions/IA_Ready`
  (params (ActionValue :type Boolean) (ElapsedSeconds :type "Float (double-precision)") (TriggeredSeconds :type "Float (double-precision)") (InputAction :type "InputAction Object Reference" :default "/Game/Blueprints/Input/Actions/IA_Ready.IA_Ready"))
  (bind _returnvalue (subsystem `EnhancedInputLocalPlayerSubsystem`))
  (:`Started`
    (`/Engine/EditorBlueprintResources/StandardMacros.DoOnce` false
      (:`Completed`
        (`self.SpawnAndPossess`)
        (set `self.Ready?` true)
        (`EnhancedInputSubsystemInterface.RemoveMappingContext` _returnvalue "/Game/Blueprints/Input/MappingContexts/IMC_Menu.IMC_Menu" (struct))
        (`EnhancedInputSubsystemInterface.AddMappingContext` _returnvalue "/Game/Blueprints/Input/MappingContexts/IMC_Ready.IMC_Ready" 0 (struct))
        (`/Game/UI/W_MainMenu.ReadyPlayer` (`self.Main Menu`) (`self.iPlayerIndex`))))))

(event `/Game/Blueprints/BPI_StartGame.ConnectToGame`
  (params (PlayerIndex :type Integer))
  (bind _output_get (set `self.iPlayerIndex` PlayerIndex))
  (`self.SetCarColor` _output_get)
  (bind _outactors (`GameplayStatics.GetAllActorsOfClass` "/Script/CinematicCamera.CineCameraActor"))
  (bind _output (`|GetArrayItem` _outactors (`self.iPlayerIndex`)))
  (`self.SetViewTargetWithBlend` self _output 0.0 "VTBlend_Linear" 0.0 false)
  (`self.K2_AttachToComponent` _output null "None" "KeepWorld" "KeepWorld" "KeepWorld" true)
  (`EnhancedInputSubsystemInterface.AddMappingContext` (subsystem `EnhancedInputLocalPlayerSubsystem`) "/Game/Blueprints/Input/MappingContexts/IMC_Menu.IMC_Menu" 0 (struct))
  (`self.SetOverlay`))

(event `/Game/Blueprints/BPI_StartGame.StartGame`
  (`EnhancedInputSubsystemInterface.AddMappingContext` (subsystem `EnhancedInputLocalPlayerSubsystem`) "/Game/Blueprints/Input/MappingContexts/IMC_Isometric.IMC_Isometric" 0 (struct))
  (bind _returnvalue (`|CreateWidget` "/Game/UI/VehicleUI.VehicleUI_C" self))
  (set `self.VehicleHud` _returnvalue)
  (`WidgetBlueprintLibrary.SetInputMode_GameOnly` self)
  (`UserWidget.AddToPlayerScreen` (`self.VehicleHud`) 0)
  (bind _aswheeled_vehicle_pawn (cast `WheeledVehiclePawn` (`self.K2_GetPawn`)))
  (set `self.Vehicle Movement Component` (`WheeledVehiclePawn.VehicleMovementComponent` _aswheeled_vehicle_pawn))
  (set `self.bShowMouseCursor` false))

(event `self.ReceiveTick`
  (params (DeltaSeconds :type "Float (single-precision)"))
  (bind _vehiclehud (`self.VehicleHud`))
  (`/Engine/EditorBlueprintResources/StandardMacros.IsValid` _vehiclehud
    (:`Is Valid`
      (`/Game/UI/VehicleUI.UpdateSpeed` _vehiclehud (`ChaosVehicleMovementComponent.GetForwardSpeed` (`self.Vehicle Movement Component`)))
      (`/Game/UI/VehicleUI.UpdateGear` (`self.VehicleHud`) (`ChaosVehicleMovementComponent.GetCurrentGear` (`self.Vehicle Movement Component`))))))

(event `EnhancedInput|/Game/Blueprints/Input/Actions/IA_ToggleCamera`
  (params (ActionValue :type Boolean) (ElapsedSeconds :type "Float (double-precision)") (TriggeredSeconds :type "Float (double-precision)") (InputAction :type "InputAction Object Reference" :default "/Game/Blueprints/Input/Actions/IA_ToggleCamera.IA_ToggleCamera"))
  (bind _returnvalue (`self.K2_GetPawn`))
  (bind _backspringarm (`/Game/Blueprints/Vehicles/Default/VehicleAdvPawn.BackSpringArm` (cast `/Game/Blueprints/Vehicles/Default/VehicleAdvPawn` (`self.K2_GetPawn`) :!pure true)))
  (:`Started`
    (if (not (`self.Switch`))
      (`/Engine/EditorBlueprintResources/StandardMacros.FlipFlop`
        (:`A`
          (set `SpringArmComponent.bInheritPitch` true _backspringarm)
          (set `SpringArmComponent.bInheritYaw` true _backspringarm)
          (set `SpringArmComponent.bInheritRoll` true _backspringarm)
          (`self.SetViewTargetWithBlend` self _returnvalue 0.0 "VTBlend_Linear" 0.0 false))
        (:`B`
          (set `SpringArmComponent.bInheritPitch` false _backspringarm)
          (set `SpringArmComponent.bInheritYaw` false _backspringarm)
          (set `SpringArmComponent.bInheritRoll` false _backspringarm)
          (bind _outactors (`GameplayStatics.GetAllActorsOfClass` "/Script/CinematicCamera.CineCameraActor"))
          (`self.SetViewTargetWithBlend` self (`|GetArrayItem` _outactors (`self.iPlayerIndex`)) 0.0 "VTBlend_Linear" 0.0 false)
          (bind _asvehicle_adv_pawn (cast `/Game/Blueprints/Vehicles/Default/VehicleAdvPawn` _returnvalue))
          (`SceneComponent.K2_SetRelativeRotation` (`/Game/Blueprints/Vehicles/Default/VehicleAdvPawn.BackSpringArm` _asvehicle_adv_pawn) (struct :`Pitch` 90.0) false false))))))

(fn `SpawnAndPossess`
  (bind _iplayerindex (`self.iPlayerIndex`))
  (bind _outactors (`GameplayStatics.GetAllActorsOfClass` "/Script/Engine.PlayerStart"))
  (`self.GetCarClass` (`|GetArrayItem` (`/Game/UI/W_MainMenu.Players Cars Types` (`self.Main Menu`)) _iplayerindex))
  (bind _returnvalue (`|SpawnActorFromClass` (`self.CarClass`) (`self.GetTransform` (`|GetArrayItem` _outactors _iplayerindex)) "AlwaysSpawn" "MultiplyWithRoot" null (`self.Team Color`) null))
  (`self.Possess` self _returnvalue)
  (bind _outactors_2 (`GameplayStatics.GetAllActorsOfClass` "/Script/CinematicCamera.CineCameraActor"))
  (bind _output (`|GetArrayItem` _outactors_2 (`self.iPlayerIndex`)))
  (`/Engine/EditorBlueprintResources/StandardMacros.IsValid` _output
    (:`Is Valid`
      (`self.SetViewTargetWithBlend` self _output 0.0 "VTBlend_Linear" 0.0 false)
      (`self.K2_AttachToComponent` _output (`/Game/Blueprints/Vehicles/Default/VehicleAdvPawn.BackSpringArm` (cast `/Game/Blueprints/Vehicles/Default/VehicleAdvPawn` (`self.K2_GetPawn`) :!pure true)) "None" "KeepWorld" "KeepWorld" "KeepWorld" false))))

(fn `UserConstructionScript`)