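; BP_Obstacle is a one-shot track trap or pickup that affects a VehicleAdvPawn according to its ObstacleType.
; The first collision overlap passes a DoOnce with no reset, then acts only on non-immune vehicles.
; Speed Pad and Slowdown apply velocity-change impulses scaled from current velocity.
; Fling applies a RandomValue-based impulse with a coin-flip sign, and Immunity calls the car's OnImmunityGained dispatcher.
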(event `self.Collision.OnComponentBeginOverlap`
  (params (OverlappedComponent :type "PrimitiveComponent Object Reference") (OtherActor :type "Actor Object Reference") (OtherComp :type "PrimitiveComponent Object Reference") (OtherBodyIndex :type Integer) (bFromSweep :type Boolean) (SweepResult :type "HitResult Structure (by ref)"))
  (`/Engine/EditorBlueprintResources/StandardMacros.DoOnce` false
    (:`Completed`
      (if (!= OtherActor self)
        (bind _asvehicle_adv_pawn (cast `/Game/Blueprints/Vehicles/Default/VehicleAdvPawn` OtherActor))
        (if (not (`/Game/Blueprints/Vehicles/Default/VehicleAdvPawn.Immune?` _asvehicle_adv_pawn))
          (switch `/Game/Blueprints/Enums/E_ObstacleType` (`self.ObstacleType`)
            (:`NewEnumerator0`
              (`self.SpeedPad` _asvehicle_adv_pawn))
            (:`NewEnumerator1`
              (`self.Fling` (`WheeledVehiclePawn.Mesh` _asvehicle_adv_pawn)))
            (:`NewEnumerator2`
              (`self.Slowdown` _asvehicle_adv_pawn))
            (:`NewEnumerator3`
              (`self.Immunity` _asvehicle_adv_pawn))))))))

(fn `Fling`
  (params (Car :type "SkeletalMeshComponent Object Reference"))
  (bind (_x _y _z) (`self.RandomValue`))
  (if (`KismetMathLibrary.RandomBool`)
    (`PrimitiveComponent.AddImpulse` Car (`KismetMathLibrary.MakeVector` (* _x 1.0) (* _y 1.0) (* _z 1.0)) "None" true)
    (else
      (`PrimitiveComponent.AddImpulse` Car (`KismetMathLibrary.MakeVector` (* _x -1.0) (* _y -1.0) (* _z -1.0)) "None" true))))

(fn `Immunity`
  (params (Car :type "/Game/Blueprints/Vehicles/Default/VehicleAdvPawn Object Reference"))
  (`/Game/Blueprints/Vehicles/Default/VehicleAdvPawn.OnImmunityGained` Car))

(fn `Slowdown`
  (params (Car :type "/Game/Blueprints/Vehicles/Default/VehicleAdvPawn Object Reference"))
  (bind _returnvalue (`self.GetVelocity` Car))
  (bind _mesh (`WheeledVehiclePawn.Mesh` Car))
  (bind (_returnvalue_x _returnvalue_y) (`KismetMathLibrary.BreakVector` (* (`KismetMathLibrary.VSizeXY` _returnvalue) (`KismetMathLibrary.InverseTransformDirection` (`self.GetTransform` Car) (`SceneComponent.GetForwardVector` _mesh)))))
  (`PrimitiveComponent.AddImpulse` _mesh (* (`KismetMathLibrary.MakeVector` _returnvalue_x _returnvalue_y (.z _returnvalue)) (0.8 -1.0 -1.0)) "None" true))

(fn `SpeedPad`
  (params (Car :type "/Game/Blueprints/Vehicles/Default/VehicleAdvPawn Object Reference"))
  (bind _returnvalue (`self.GetVelocity` Car))
  (bind _mesh (`WheeledVehiclePawn.Mesh` Car))
  (bind (_returnvalue_x _returnvalue_y) (`KismetMathLibrary.BreakVector` (* (`KismetMathLibrary.VSizeXY` _returnvalue) (`SceneComponent.GetForwardVector` _mesh))))
  (`PrimitiveComponent.AddImpulse` _mesh (* (`KismetMathLibrary.MakeVector` _returnvalue_x _returnvalue_y (.z _returnvalue)) (1.7 1.0 1.6)) "None" true))

(fn `UserConstructionScript`)